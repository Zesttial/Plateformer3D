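; BP_CanonBullet is a cannon projectile that knocks the player back and costs a life on hit.
; When its collider begins an overlap, it resets its lifespan to the initial value, then continues only for the third-person character.
; It launches that character along the bullet's velocity, scaled by PushForce with an upward boost, overriding existing velocity.
; It then calls LoseLife on the third-person game mode and destroys itself.
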(event OnComponentBeginOverlap(Bullet_Collider)
  (params (OverlappedComponent :type Primitive%20Component%20Object%20Reference) (OtherActor :type Actor%20Object%20Reference) (OtherComp :type Primitive%20Component%20Object%20Reference) (OtherBodyIndex :type Integer) (bFromSweep :type Boolean) (SweepResult :type Hit%20Result%20Structure%20%28by%20ref%29))
  (Actor|SetLifeSpan (Variables|Actor|GetInitialLifeSpan))
  (bind _asbp_third_person_character (Utilities|Casting|CastToBP_ThirdPersonCharacter OtherActor))
  (Character|LaunchCharacter _asbp_third_person_character (+ (* (Math|Vector|Normalize (Transformation|GetVelocity)) (Variables|Default|GetPushForce)) "0.000000,0.000000,500.000000") true true)
  (bind _asbp_third_person_game_mode (Utilities|Casting|CastToBP_ThirdPersonGameMode (Game|GetGameMode)))
  (Default|LoseLife _asbp_third_person_game_mode)
  (Actor|DestroyActor))

(event EventBeginPlay)

(event Collision|EventActorBeginOverlap
  (params (OtherActor :type Actor%20Object%20Reference)))

(event EventTick
  (params (DeltaSeconds :type Float%20%28single-precision%29)))

(fn ConstructionScript)